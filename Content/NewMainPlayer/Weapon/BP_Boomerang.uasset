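; Throwable returning axe for the player character that flies out, lands where it hits and arcs back to the hand.
; BeThrowOut detaches it and adds a zero-gravity projectile movement component along the throw direction.
; A hit snaps it to the impact point with a sound, unless it is returning.
; AxeReturn runs a distance-scaled timeline toward the live hand socket, curving sideways, then notifies NewThirdPersonCharacter.
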(event OnComponentHit(Axe)
  (params (HitComponent :type Primitive%20Component%20Object%20Reference) (OtherActor :type Actor%20Object%20Reference) (OtherComp :type Primitive%20Component%20Object%20Reference) (NormalImpulse :type Vector :default "0, 0, 0") (Hit :type Hit%20Result%20Structure%20%28by%20ref%29))
  (if (not (Variables|Default|GetReturn))
    (CallFunction|LandedEvent Hit)))

(event Custom|GravityFix
  (bind _projectile (Variables|Default|GetProjectile))
  (Variables|/Script/Engine.ProjectileMovementComponent|SetProjectileGravityScale _projectile 0.0)
  (Utilities|FlowControl|Delay 0.3)
  (Variables|/Script/Engine.ProjectileMovementComponent|SetProjectileGravityScale _projectile 0.0))

(event Custom|AxeReturn
  (if (Variables|Default|GetHitSometing)
    _
    (else
      (Variables|Default|SetThrown true)))
  (Variables|Default|SetHitSometing false)
  (CallFunction|ReadReturn)
  (bind (_direction _axereturnpre _rightline) (Timeline|AxeReturnCurve PlayFromStart)
    (:Update
      (CallFunction|CalculateAxeLoc _axereturnpre _rightline))
    (:Finished
      (CallFunction|AxeReturnedFinish))))

(event EventTick
  (params (DeltaSeconds :type Float%20%28single-precision%29))
  (CallFunction|UpdataHandLoc))

(event EventBeginPlay
  (Components|Activation|SetActive (Variables|Default|GetNiagara) false false)
  (Components|Activation|SetActive (Variables|Default|GetNiagara2) false false)
  (Components|Activation|SetActive (Variables|Default|GetNiagara3) false false)
  (Collision|SetCollisionEnabled (Variables|Default|GetBox) "NoCollision"))

(fn ConstructionScript)

(fn BeThrowOut
  (params (Dir :type Vector) (Thrower :type Character%20Object%20Reference))
  (Variables|Default|SetThrowDir Dir)
  (Variables|Default|SetThrower Thrower)
  (Variables|Default|SetThrown true)
  (Collision|SetCollisionEnabled (Variables|Default|GetBox) "QueryAndPhysics")
  (Transformation|DetachFromActor "KeepWorld" "KeepWorld" "KeepWorld")
  (Collision|SetCollisionResponsetoChannel (Variables|Default|GetAxe) "ECC_WorldStatic" "ECR_Block")
  (bind _returnvalue (AddComponent|AddProjectileMovementComponent))
  (bind _output_get (Variables|Default|SetProjectile _returnvalue))
  (Game|Components|ProjectileMovement|SetVelocityinLocalSpace _output_get (* (Variables|Default|GetThrowDir) (Variables|Default|GetThrowForce)))
  (Components|Activation|SetActive _output_get true false)
  (Transformation|SetActorRelativeRotation (Pawn|GetControlRotation (Variables|Default|GetThrower) :!class /Script/Engine.Pawn))
  (Components|Activation|SetActive (Variables|Default|GetNiagara) true false)
  (CallFunction|GravityFix))

(fn LandedEvent
  (params (Hit :type Hit%20Result%20Structure))
  (bind (_bblockinghit _binitialoverlap _time _distance _location _impactpoint _normal) (Collision|BreakHitResult Hit))
  (bind _returnvalue (Math|Vector|DotProduct _normal "0, 0,1.000000"))
  (Variables|Default|SetHitSometing true)
  (Variables|Default|SetThrown false)
  (Variables|Default|SetHitWall (<= (Math|Float|Absolute(Float) _returnvalue) 0.5))
  (Variables|Default|SetHitFloor (> _returnvalue 0.5))
  (Audio|PlaySoundatLocation "/Game/Original/StarterContent/Audio/Explosion_Cue.Explosion_Cue" _location "0, 0, 0" 1.0 1.0 0.0 0 0 0 0)
  (Transformation|SetActorLocationAndRotation self _location (Math|Rotator|MakeRotator 0.0 1.8e+02 (.yaw (Math|Conversions|RotationFromXVector (* (Math|Vector|Normalize (Transformation|GetVelocity)) -1.0)))))
  (Components|Activation|SetActive (Variables|Default|GetNiagara) false false))

(fn CalculateAxeLoc
  (params (AxeReturnPre :type Float%20%28double-precision%29) (RightLine :type Float%20%28double-precision%29))
  (Variables|Default|SetAxe%20Return%20Pre AxeReturnPre)
  (Transformation|SetActorLocation (+ (Variables|Default|GetAxeInitLoc) (* (- (Variables|Default|GetRHandLoc) (Variables|Default|GetAxeInitLoc)) (Variables|Default|GetAxe%20Return%20Pre)) (* (Variables|Default|GetRightVector) (* (Variables|Default|GetDistanceToRate) RightLine 5e+02))) false false))

(fn AxeReturnedFinish
  (Variables|Default|SetHitSometing false)
  (Variables|Default|SetThrown false)
  (Variables|Default|SetReturn false)
  (bind _asnew_third_person_character (Utilities|Casting|CastToNewThirdPersonCharacter (Variables|Default|GetThrower)))
  (Default|AxeReturned _asnew_third_person_character))

(fn UpdataHandLoc
  (if (Variables|Default|GetReturn)
    (Variables|Default|SetRHandLoc (Transformation|GetSocketLocation (Variables|/Script/Engine.Character|GetMesh (Variables|Default|GetThrower)) "Axesocket"))))

(fn ReadReturn
  (Variables|Default|SetReturn true)
  (Variables|Default|SetAxeInitLoc (Transformation|GetActorLocation))
  (Variables|Default|SetDistanceToRate (/ (Math|Vector|VectorLength (- (Transformation|GetSocketLocation (Variables|/Script/Engine.Character|GetMesh (Variables|Default|GetThrower)) "Axesocket") (Variables|Default|GetAxeInitLoc))) 6e+03))
  (Components|Timeline|SetPlayRate (Variables|Default|GetAxeReturnCurve) (/ 1.0 (Variables|Default|GetDistanceToRate)))
  (Variables|Default|SetRightVector (Math|Vector|Normalize (Math|Vector|CrossProduct (- (Transformation|GetSocketLocation (Variables|/Script/Engine.Character|GetMesh (Variables|Default|GetThrower)) "Axesocket") (Variables|Default|GetAxeInitLoc)) "0, 0,1.000000")))
  (Components|Activation|SetActive (Variables|Default|GetNiagara2) true false)
  (Components|Activation|SetActive (Variables|Default|GetNiagara) false false)
  (Collision|SetCollisionEnabled (Variables|Default|GetBox) "NoCollision"))

(fn NoWeapon
  (params (Thrower :type Character%20Object%20Reference))
  (Variables|Default|SetThrower Thrower)
  (Transformation|DetachFromActor "KeepWorld" "KeepWorld" "KeepWorld")
  (Collision|SetCollisionResponsetoChannel (Variables|Default|GetAxe) "ECC_WorldStatic" "ECR_Block"))