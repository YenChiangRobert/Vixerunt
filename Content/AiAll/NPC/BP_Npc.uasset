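; NPC Blueprint for a wanderer that talks when the player character enters its Talk trigger.
; Overlap start plays a 2D voice sound, loops the talk animation on Mesh and creates and shows a WG_NpcTalk widget.
; Overlap end removes the widget, restores the looping idle animation and hides the SkeletalMesh component in game.
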(event OnComponentBeginOverlap(talk)
  (params (OverlappedComponent :type Primitive%20Component%20Object%20Reference) (OtherActor :type Actor%20Object%20Reference) (OtherComp :type Primitive%20Component%20Object%20Reference) (OtherBodyIndex :type Integer) (bFromSweep :type Boolean) (SweepResult :type Hit%20Result%20Structure%20%28by%20ref%29))
  (Utilities|Casting|CastToNewThirdPersonCharacter OtherActor)
  (Audio|PlaySound2D "/Game/sound/NPC_講話聲.NPC_講話聲" 1.0 1.0 0.0 0 0)
  (Components|Animation|PlayAnimation (Variables|Character|GetMesh) "/Game/AiAll/NPC/talk/NPC_流浪者_對話_Anim.NPC_流浪者_對話_Anim" true)
  (bind _returnvalue (UserInterface|CreateWidget "/Game/UI/WG_NpcTalk.WG_NpcTalk_C"))
  (bind _output_get (Variables|Default|Setuser _returnvalue))
  (UserInterface|Viewport|AddtoViewport _output_get 0)
  (Widget|SetVisibility _output_get "Visible"))

(event OnComponentEndOverlap(talk)
  (params (OverlappedComponent :type Primitive%20Component%20Object%20Reference) (OtherActor :type Actor%20Object%20Reference) (OtherComp :type Primitive%20Component%20Object%20Reference) (OtherBodyIndex :type Integer))
  (Utilities|FlowControl|Sequence
    (:then_0
      (Utilities|Casting|CastToNewThirdPersonCharacter OtherActor)
      (Widget|RemovefromParent (Variables|Default|Getuser))
      (Components|Animation|PlayAnimation (Variables|Character|GetMesh) "/Game/AiAll/NPC/idle/NPC_流浪者_待機_Anim.NPC_流浪者_待機_Anim" true))
    (:then_1
      (Utilities|Casting|CastToNewThirdPersonCharacter OtherActor)
      (Development|SetHiddeninGame (Variables|Default|GetSkeletalMesh) true false))))

(event EventBeginPlay)

(event Collision|EventActorBeginOverlap
  (params (OtherActor :type Actor%20Object%20Reference)))

(event EventTick
  (params (DeltaSeconds :type Float%20%28single-precision%29)))

(fn ConstructionScript)