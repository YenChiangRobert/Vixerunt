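; BP_ToCG is a level transition trigger that opens the HomeCG level once no required objects remain in the level.
; When a NewThirdPersonCharacter overlaps it, it searches for all BP_Check, BP_pickupBook and BP_pickupphoto actors.
; The level opens only if all three searches return empty, so progress is inferred from actor absence rather than stored state.
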(event EventBeginPlay)

(event Collision|EventActorBeginOverlap
  (params (OtherActor :type Actor%20Object%20Reference))
  (Utilities|Casting|CastToNewThirdPersonCharacter OtherActor)
  (bind _outactors (Actor|GetAllActorsOfClass "/Game/object/BP/BP_Check.BP_Check_C"))
  (bind _outactors_2 (Actor|GetAllActorsOfClass "/Game/object/BP/BP_pickupBook.BP_pickupBook_C"))
  (bind _outactors_3 (Actor|GetAllActorsOfClass "/Game/object/BP/BP_pickupphoto.BP_pickupphoto_C"))
  (if (and (and (== (Utilities|Array|Length _outactors) 0) (== (Utilities|Array|Length _outactors_2) 0)) (== (Utilities|Array|Length _outactors_3) 0))
    (Game|OpenLevel(byName) "HomeCG")))

(event EventTick
  (params (DeltaSeconds :type Float%20%28single-precision%29)))

(fn ConstructionScript)