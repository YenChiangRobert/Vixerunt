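; BP_pickupphoto is a photo pickup that shows a prompt when the player is nearby and opens a photo screen when taken.
; Box overlap with NewThirdPersonCharacter adds a WG_ShowEBook widget to the viewport and removes it on exit.
; The TAKEBOOK event removes the prompt, destroys the actor, shows WG_tPhoto, then pauses the game with a visible cursor and UI-only input.
; Nothing in this graph calls TAKEBOOK.
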(event OnComponentBeginOverlap(Box)
  (params (OverlappedComponent :type Primitive%20Component%20Object%20Reference) (OtherActor :type Actor%20Object%20Reference) (OtherComp :type Primitive%20Component%20Object%20Reference) (OtherBodyIndex :type Integer) (bFromSweep :type Boolean) (SweepResult :type Hit%20Result%20Structure%20%28by%20ref%29))
  (Utilities|Casting|CastToNewThirdPersonCharacter OtherActor)
  (bind _returnvalue (UserInterface|CreateWidget "/Game/object/UI/ShowE/WG_ShowEBook.WG_ShowEBook_C"))
  (bind _output_get (Variables|Default|SetTarget _returnvalue))
  (UserInterface|Viewport|AddtoViewport _output_get 0))

(event OnComponentEndOverlap(Box)
  (params (OverlappedComponent :type Primitive%20Component%20Object%20Reference) (OtherActor :type Actor%20Object%20Reference) (OtherComp :type Primitive%20Component%20Object%20Reference) (OtherBodyIndex :type Integer))
  (Utilities|Casting|CastToNewThirdPersonCharacter OtherActor)
  (Widget|RemovefromParent (Variables|Default|GetTarget)))

(event EventBeginPlay)

(event Collision|EventActorBeginOverlap
  (params (OtherActor :type Actor%20Object%20Reference)))

(event EventTick
  (params (DeltaSeconds :type Float%20%28single-precision%29)))

(event EventTAKEBOOK
  (bind _returnvalue (Game|GetPlayerController 0))
  (Widget|RemovefromParent (Variables|Default|GetTarget))
  (Actor|DestroyActor)
  (bind _returnvalue_2 (UserInterface|CreateWidget "/Game/object/UI/Page/Photo/WG_tPhoto.WG_tPhoto_C"))
  (bind _output_get (Variables|Default|SetTarget _returnvalue_2))
  (UserInterface|Viewport|AddtoViewport _output_get 0)
  (Widget|SetVisibility (Variables|Default|GetTarget) "Visible")
  (Variables|/Script/Engine.PlayerController|SetbShowMouseCursor _returnvalue true)
  (Input|SetInputModeUIOnly _returnvalue 0 "DoNotLock")
  (Game|SetGamePaused true))

(fn ConstructionScript)