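; BP_pickup1 is a health pickup actor that shows an interaction prompt when the player character is near.
; Box overlap with NewThirdPersonCharacter creates the WG_ShowE1 widget and adds it to the viewport, and leaving removes it.
; The TAKEOBJ event, not called within this Blueprint, removes the prompt, destroys the actor and sets the player's Health to a fixed value.
; Disconnected leftover nodes for player UI, health and photo widgets never run.
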(event OnComponentBeginOverlap(Box)
  (params (OverlappedComponent :type Primitive%20Component%20Object%20Reference) (OtherActor :type Actor%20Object%20Reference) (OtherComp :type Primitive%20Component%20Object%20Reference) (OtherBodyIndex :type Integer) (bFromSweep :type Boolean) (SweepResult :type Hit%20Result%20Structure%20%28by%20ref%29))
  (bind _asnew_third_person_character (Utilities|Casting|CastToNewThirdPersonCharacter OtherActor))
  (bind _returnvalue (UserInterface|CreateWidget "/Game/object/UI/ShowE/WG_ShowE1.WG_ShowE1_C"))
  (bind _output_get (Variables|Default|SetTarget _returnvalue))
  (UserInterface|Viewport|AddtoViewport _output_get 0))

(event OnComponentEndOverlap(Box)
  (params (OverlappedComponent :type Primitive%20Component%20Object%20Reference) (OtherActor :type Actor%20Object%20Reference) (OtherComp :type Primitive%20Component%20Object%20Reference) (OtherBodyIndex :type Integer))
  (Utilities|Casting|CastToNewThirdPersonCharacter OtherActor)
  (Widget|RemovefromParent (Variables|Default|GetTarget)))

(event EventBeginPlay)

(event Collision|EventActorBeginOverlap
  (params (OtherActor :type Actor%20Object%20Reference)))

(event EventTick
  (params (DeltaSeconds :type Float%20%28single-precision%29)))

(event EventTAKEOBJ
  (Widget|RemovefromParent (Variables|Default|GetTarget))
  (Actor|DestroyActor)
  (bind _asnew_third_person_character (Utilities|Casting|CastToNewThirdPersonCharacter (Game|Player|GetPlayerPawn 0)))
  (Variables|/Game/NewMainPlayer/NewThirdPersonCharacter.NewThirdPersonCharacter_C|SetHealth _asnew_third_person_character 1e+02))

(fn ConstructionScript)