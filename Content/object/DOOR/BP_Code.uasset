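; BP_Code is a trigger actor in the door object set that brings up the UMG_Code screen when the player walks into it.
; When NewThirdPersonCharacter overlaps its Box, it proceeds only if no BP_Check2 actors exist in the level.
; It then creates and shows the widget, enables the mouse cursor, switches to UI-only input and pauses the game.
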(event OnComponentBeginOverlap(Box)
  (params (OverlappedComponent :type Primitive%20Component%20Object%20Reference) (OtherActor :type Actor%20Object%20Reference) (OtherComp :type Primitive%20Component%20Object%20Reference) (OtherBodyIndex :type Integer) (bFromSweep :type Boolean) (SweepResult :type Hit%20Result%20Structure%20%28by%20ref%29))
  (bind _returnvalue (Game|GetPlayerController 0))
  (Utilities|Casting|CastToNewThirdPersonCharacter OtherActor)
  (bind _outactors (Actor|GetAllActorsOfClass "/Game/object/BP/BP_Check2.BP_Check2_C"))
  (if (== (Utilities|Array|Length _outactors) 0)
    (bind _returnvalue_2 (UserInterface|CreateWidget "/Game/object/DOOR/UMG_Code.UMG_Code_C"))
    (bind _output_get (Variables|Default|Settarget _returnvalue_2))
    (UserInterface|Viewport|AddtoViewport _output_get 0)
    (Widget|SetVisibility _output_get "Visible")
    (Variables|/Script/Engine.PlayerController|SetbShowMouseCursor _returnvalue true)
    (Input|SetInputModeUIOnly _returnvalue 0 "DoNotLock")
    (Game|SetGamePaused true)))

(event EventBeginPlay)

(event Collision|EventActorBeginOverlap
  (params (OtherActor :type Actor%20Object%20Reference)))

(event EventTick
  (params (DeltaSeconds :type Float%20%28single-precision%29)))

(fn ConstructionScript)