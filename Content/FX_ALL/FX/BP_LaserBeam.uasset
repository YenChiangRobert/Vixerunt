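; BP_LaserBeam is a laser beam actor that extends along its forward vector and stops at whatever blocks it.
; Each tick it traces on the Camera channel, with per-frame debug drawing, setting the beam effect's end and showing the impact effect at hits.
; Distance snaps back to the hit length, then grows over time up to a cap, so the beam re-extends gradually once unblocked.
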(event EventTick
  (params (DeltaSeconds :type Float%20%28single-precision%29))
  (bind _returnvalue (Transformation|GetActorLocation))
  (bind _fx_laserimpact (Variables|Default|GetFX_LaserImpact))
  (Utilities|FlowControl|Sequence
    (:then_0
      (Variables|Default|SetTraceEnd (+ _returnvalue (* (Transformation|GetActorForwardVector) (Variables|Default|GetDistance))))
      (bind _outhit (Collision|LineTraceByChannel _returnvalue (+ _returnvalue (* (Transformation|GetActorForwardVector) (Variables|Default|GetDistance))) "TraceTypeQuery2" false 0 "ForOneFrame"))
      (Variables|Default|SetHit (.bBlockingHit (Collision|BreakHitResult _outhit)))
      (Variables|Default|SetHitLocation (.Location (Collision|BreakHitResult _outhit)))
      (Effects|Components|ParticleSystem|SetVectorParameter (Variables|Default|GetFX_LaserBeam) "LaserEnd" (select (Variables|Default|GetHit) (Variables|Default|GetHitLocation) (Variables|Default|GetTraceEnd)))
      (Rendering|SetVisibility _fx_laserimpact (Variables|Default|GetHit) false)
      (Transformation|SetWorldLocation _fx_laserimpact (Variables|Default|GetHitLocation) false false)
      (if (Variables|Default|GetHit)
        (Variables|Default|SetDistance (Math|Vector|VectorLength (- (Variables|Default|GetHitLocation) (Transformation|GetActorLocation))))))
    (:then_1
      (if (< (Variables|Default|GetDistance) 5e+03)
        (Variables|Default|SetDistance (+ (Variables|Default|GetDistance) (* DeltaSeconds 5e+02)))))))

(fn ConstructionScript)