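; BP_Poison is a poison spit effect actor that traces along its forward vector every tick on the Camera channel.
; The trace length grows over time up to a cap and snaps back to any blocking hit.
; The spit beam's LaserEnd follows the trace end or impact, where the poison effect shows.
; Each hit tick also spawns a fading blood decal, noted in a comment as not yet working.
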(event EventTick
  (params (DeltaSeconds :type Float%20%28single-precision%29))
  (bind _returnvalue (Transformation|GetActorLocation))
  (bind _fx_poison (Variables|Default|GetFX_Poison))
  (Utilities|FlowControl|Sequence
    (:then_0
      (Variables|Default|SetTraceEnd (+ _returnvalue (* (Transformation|GetActorForwardVector) (Variables|Default|GetDistance))))
      (bind _outhit (Collision|LineTraceByChannel _returnvalue (+ _returnvalue (* (Transformation|GetActorForwardVector) (Variables|Default|GetDistance))) "TraceTypeQuery2" false 0 "ForOneFrame"))
      (Variables|Default|SetHit (.bBlockingHit (Collision|BreakHitResult _outhit)))
      (Variables|Default|SetHitLocation (.Location (Collision|BreakHitResult _outhit)))
      (Effects|Components|ParticleSystem|SetVectorParameter (Variables|Default|GetFX_Spit) "LaserEnd" (select (Variables|Default|GetHit) (Variables|Default|GetHitLocation) (Variables|Default|GetTraceEnd)))
      (Rendering|SetVisibility _fx_poison (Variables|Default|GetHit) false)
      (Transformation|SetWorldLocation _fx_poison (Variables|Default|GetHitLocation) false false)
      (if (Variables|Default|GetHit)
        (Variables|Default|SetDistance (Math|Vector|VectorLength (- (Variables|Default|GetHitLocation) (Transformation|GetActorLocation))))
        ;[1 1 1] 沒反應，再研究
        (bind _returnvalue_2 (Rendering|Decal|SpawnDecalatLocation "/Game/FX/FX_Material/M_BloodDecal.M_BloodDecal" "0, 0, 0" (Variables|Default|GetHitLocation) "-90.000000,0.000000,0.000000" 0.0))
        (Rendering|Components|Decal|SetFadeOut _returnvalue_2 3.0 5.0 true)))
    (:then_1
      (if (< (Variables|Default|GetDistance) 5e+03)
        (Variables|Default|SetDistance (+ (Variables|Default|GetDistance) (* DeltaSeconds 5e+02)))))))

(fn ConstructionScript)